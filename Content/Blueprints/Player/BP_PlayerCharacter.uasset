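; Player character Blueprint that plays weapon equip, unequip and fire animations in response to its WeaponComponent.
; BeginPlay binds to the component's weapon-changed and fired events, and each handler selects an animation by the current weapon's type.
; Weapon changes play montages through the AnimInstance, while firing calls PlayAnimation directly on the mesh.
; Only Pistol and Rifle have equip and fire animations; Shotgun slots are empty.
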(event `self.ReceiveBeginPlay`
  (bind _weaponcomponent (`self.WeaponComponent`))
  (add `WeaponComponent.OnWeaponChanged` _weaponcomponent (delegate `CustomEvent_OnWeaponChanged`))
  (add `WeaponComponent.OnFired` _weaponcomponent (delegate `CustomEvent_OnFired`)))

(event `CustomEvent_OnWeaponChanged`
  (params (NewWeapon :type "WeaponDataAsset Object Reference"))
  (bind _returnvalue (`SkeletalMeshComponent.GetAnimInstance` (`self.Mesh`)))
  (bind (_weapondata_damage _weapondata_firerate _weapondata_totalammo _weapondata_bulletspeed _weapondata_projectileclass _weapondata_weapontype) (break `WeaponData` (`WeaponDataAsset.WeaponData` (`WeaponUser.GetCurrentWeapon` (`self.WeaponComponent`)))))
  (`/Engine/EditorBlueprintResources/StandardMacros.IsValid` NewWeapon
    (:`Is Valid`
      (`AnimInstance.Montage_Play` _returnvalue (select `EWeaponType` _weapondata_weapontype :`None` "/Game/Characters/Heroes/Mannequin/Animations/Actions/AM_MM_Generic_Unequip.AM_MM_Generic_Unequip" :`Pistol` "/Game/Weapons/Pistol/Animations/AM_MM_Pistol_Equip.AM_MM_Pistol_Equip" :`Rifle` "/Game/Weapons/Rifle/Animations/AM_MM_Rifle_Equip.AM_MM_Rifle_Equip" :`Unarmed` "/Game/Characters/Heroes/Mannequin/Animations/Actions/AM_MM_Generic_Unequip.AM_MM_Generic_Unequip" :!type "AnimMontage Object Reference") 1.0 "MontageLength" 0.0 true))
    (:`Is Not Valid`
      (`AnimInstance.Montage_Play` _returnvalue "/Game/Characters/Heroes/Mannequin/Animations/Actions/AM_MM_Generic_Unequip.AM_MM_Generic_Unequip" 1.0 "MontageLength" 0.0 true))))

(event `CustomEvent_OnFired`
  (bind (_weapondata_damage _weapondata_firerate _weapondata_totalammo _weapondata_bulletspeed _weapondata_projectileclass _weapondata_weapontype) (break `WeaponData` (`WeaponDataAsset.WeaponData` (`WeaponUser.GetCurrentWeapon` (`self.WeaponComponent`)))))
  (`SkeletalMeshComponent.PlayAnimation` (`self.Mesh`) (select `EWeaponType` _weapondata_weapontype :`Pistol` "/Game/Weapons/Pistol/Animations/AM_MM_Pistol_Fire.AM_MM_Pistol_Fire" :`Rifle` "/Game/Weapons/Rifle/Animations/AM_MM_Rifle_Fire.AM_MM_Rifle_Fire" :!type "AnimationAsset Object Reference") false))

(fn `UserConstructionScript`)